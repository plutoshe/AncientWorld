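; BP_BuildingDesk is an interactable desk that sends the player to the BuildingSystem level.
; Tick accumulates the time elapsed in FTimeHasBeen.
; On BPInteract it prints a debug string, opens the level by name, then adds that time to MusicEndSecs on bp_AncientWorldGameInstance, apparently to carry music position across levels.
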(event EventBeginPlay)

(event Collision|EventActorBeginOverlap
  (params (OtherActor :type Actor%20Object%20Reference)))

(event EventTick
  (params (DeltaSeconds :type Float%20%28single-precision%29))
  (Variables|Default|SetfTimeHasBeen (+ (Variables|Default|GetfTimeHasBeen) DeltaSeconds)))

(event EventBPInteract
  (Development|PrintString "Press building desk")
  (Game|OpenLevel(byName) "BuildingSystem")
  (bind _asbp_ancient_world_game_instance (Utilities|Casting|CastTobp_AncientWorldGameInstance (Game|GetGameInstance)))
  (Variables|/Game/Blueprint/bp_AncientWorldGameInstance.bp_AncientWorldGameInstance_C|SetMusicEndSecs _asbp_ancient_world_game_instance (+ (Variables|/Game/Blueprint/bp_AncientWorldGameInstance.bp_AncientWorldGameInstance_C|GetMusicEndSecs _asbp_ancient_world_game_instance) (Variables|Default|GetfTimeHasBeen))))

(fn ConstructionScript)