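; BP_LevelManager handles level switching from the keyboard and streams in the BosonWindow level on BeginPlay with a blocking load.
; It enables input for the first player controller and caches the BP_AncientWorldGameState.
; Z and X each save the player pawn's transform to that game state, then Z opens the BuildingSystem level by name and X calls LoadLevel for BosonWindow.
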(event EventBeginPlay
  (Input|EnableInput (Game|GetPlayerController 0))
  (bind _asbp_ancient_world_game_state (Utilities|Casting|CastToBP_AncientWorldGameState (Game|GetGameState)))
  (Variables|Default|SetWorldGameState _asbp_ancient_world_game_state)
  (Game|LoadStreamLevel(byName) "BosonWindow" true true))

(event Input|KeyboardEvents|Z
  (params (Key :type Key%20Structure))
  (:Pressed
    (Variables|/Game/Blueprint/BP_AncientWorldGameState.BP_AncientWorldGameState_C|SetStoredPlayerTransform (Variables|Default|GetWorldGameState) (Transformation|GetActorTransform (Game|Player|GetPlayerPawn 0)))
    (Game|OpenLevel(byName) "BuildingSystem")))

(event Input|KeyboardEvents|X
  (params (Key :type Key%20Structure))
  (:Pressed
    (Variables|/Game/Blueprint/BP_AncientWorldGameState.BP_AncientWorldGameState_C|SetStoredPlayerTransform (Variables|Default|GetWorldGameState) (Transformation|GetActorTransform (Game|Player|GetPlayerPawn 0)))
    (Class|LevelManager|LoadLevel "BosonWindow")))

(fn ConstructionScript)