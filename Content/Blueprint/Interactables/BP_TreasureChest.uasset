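; BP_TreasureChest is an interactable treasure chest that pays out gold pieces a single time.
; On BPInteract it checks and sets a disabled flag so it cannot be reused, then marks itself opened and hides its outline mesh.
; It then loops to spawn several BP_GoldPieceUp actors slightly above its location, ignoring collision.
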(event EventBeginPlay)

(event Collision|EventActorBeginOverlap
  (params (OtherActor :type Actor%20Object%20Reference)))

(event EventTick
  (params (DeltaSeconds :type Float%20%28single-precision%29)))

(event EventBPInteract
  (if (not (Variables|Default|Getm_bInteractDisabled))
    (Variables|Default|Setm_bInteractDisabled true)
    (Variables|Gameplay|SetbOpened true)
    (Rendering|SetVisibility (Variables|Default|GetOutlineMesh) false false)
    (for _index (range 0 2)
      (Game|SpawnActorfromClass "/Game/Blueprint/PickItem/BP_GoldPieceUp.BP_GoldPieceUp_C" (Math|Transform|MakeTransform (+ (Transformation|GetActorLocation) (* (Math|Vector|VectorUp) 20)) "0, 0, 0" "1,1,1") "AlwaysSpawn" 0 0))))

(fn ConstructionScript)