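; Player controller base Blueprint that handles cursor hover outlines on interactable items (APInteractItemBase).
; Each Tick traces under the cursor on the Visibility channel and, when no such item is hit, hides the stored item's outline mesh and clears it.
; The logic that shows the outline and stores the hovered item is disconnected, so the graph only performs the clearing step.
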(event EventTick
  (params (DeltaSeconds :type Float%20%28single-precision%29))
  (bind _asapinteract_item_base (Utilities|Casting|CastToAPInteractItemBase (.hitactor (.HitResult (Game|Player|GetHitResultUnderCursorbyChannel "TraceTypeQuery1" true))))
    (:CastFailed
      (Utilities|IsValid (Variables|Default|GetmCurrentHitItem)
        (:Is%20Valid
          (Rendering|SetVisibility (Variables|/Script/AncientWorld.APInteractItemBase|GetOutlineMesh (Variables|Default|GetmCurrentHitItem)) false false)
          (Variables|/Script/AncientWorld.APInteractItemBase|Setm_bHasOutline (Variables|Default|GetmCurrentHitItem) false)
          (Variables|Default|SetmCurrentHitItem 0))))))

(fn ConstructionScript)