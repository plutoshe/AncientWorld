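; BP_VenturePawn is a player pawn with a building-focus camera toggle, HUD inventory and vertical swimming.
; On BeginPlay it caches BP_APGameMode, creates the HUD, then anchors an InventoryWindow fed by its InventoryComp near the bottom center of the HUD canvas.
; Z blends the view between the pawn and the game mode's target viewer.
; BPSwimNormal applies axis-scaled vertical velocity impulses while swimming.
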(event EventBeginPlay
  (bind _inventorycomp (Variables|Default|GetInventoryComp))
  (Utilities|FlowControl|Sequence
    (:then_0
      (bind _asbp_apgame_mode (Utilities|Casting|CastToBP_APGameMode (Game|GetGameMode)))
      (Variables|Default|SetGM _asbp_apgame_mode)
      (bind _returnvalue (UserInterface|CreateWidget "/Game/UI/BP_HUD.BP_HUD_C"))
      (bind _output_get (Variables|Default|SetHUDWidget _returnvalue))
      (UserInterface|Viewport|AddtoViewport _output_get 0))
    (:then_1
      ;[1 1 1] Inventory
      (bind _returnvalue_2 (Class|InventoryComponent|GetNumOfSlots _inventorycomp))
      (bind _returnvalue_3 (Class|InventoryComponent|GetInventory _inventorycomp))
      (bind _returnvalue_4 (UserInterface|CreateWidget "/Game/UI/InventorySystem/InventoryUI/InventoryWindow.InventoryWindow_C" (Game|GetPlayerController 0) _returnvalue_3 _returnvalue_2 _inventorycomp))
      (UserInterface|Viewport|AddtoViewport _returnvalue_4 0)
      (bind _returnvalue_5 (Class|CanvasPanel|AddChildtoCanvas (Variables|/Game/UI/InventorySystem/InventoryUI/HUD.HUD_C|GetHudCanvas (Variables|Default|GetHUDWidget)) _returnvalue_4))
      (Class|CanvasPanelSlot|SetAutoSize _returnvalue_5 true)
      (Class|CanvasPanelSlot|SetAlignment _returnvalue_5 "(X=0.500000,Y=0.000000)")
      (Class|CanvasPanelSlot|SetAnchors _returnvalue_5 (Utilities|Struct|MakeAnchors "(X=0.500000,Y=0.900000)" "(X=0.500000,Y=0.900000)")))))

(event EventBPSwimNormal
  (params (axis :type Float%20%28single-precision%29))
  (bind _charactermovement (Variables|Character|GetCharacterMovement))
  (if (AI|Components|NavMovement|IsSwimming _charactermovement :!class /Script/Engine.NavMovementComponent)
    (Physics|AddImpulse _charactermovement (* (Math|Vector|MakeVector 0.0 0.0 axis) "0, 0,25.000000") true)))

(event Input|KeyboardEvents|Z
  (params (Key :type Key%20Structure))
  (bind _returnvalue (Game|GetPlayerController 0))
  (:Pressed
    (if (Variables|Default|GetbFocusInBuilding)
      (Game|Player|SetViewTargetwithBlend _returnvalue self 0.5 "VTBlend_Linear" 0.0 false)
      (Variables|Default|SetbFocusInBuilding false)
      (else
        (bind _targetviewref (Default|GetTargetViewer (Variables|Default|GetGM)))
        (Game|Player|SetViewTargetwithBlend _returnvalue _targetviewref 0.5 "VTBlend_Linear" 0.0 false)
        (Variables|Default|SetbFocusInBuilding true)))))

(fn ConstructionScript)