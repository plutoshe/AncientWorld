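; BP_TargetViewer is an actor that follows the player pawn at an offset while orienting itself toward a target actor.
; BeginPlay caches player 0's controlled pawn as a BP_PlayerBase.
; Each Tick turns the vector to Target into a quaternion-derived rotation, then snaps the location to the player's position plus PositionOffset.
; Rotation is computed before the move, so it uses the actor's pre-move position.
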(event EventBeginPlay
  (bind _asbp_player_base (Utilities|Casting|CastToBP_PlayerBase (Pawn|GetControlledPawn (Game|GetPlayerController 0))))
  (Variables|Default|SetFollowedPlayer _asbp_player_base))

(event Collision|EventActorBeginOverlap
  (params (OtherActor :type Actor%20Object%20Reference)))

(event EventTick
  (params (DeltaSeconds :type Float%20%28single-precision%29))
  (Transformation|SetActorRotation (Class|KismetMathLibrary|QuatRotator (Class|KismetMathLibrary|ToQuaterion(Vector) (- (Transformation|GetActorLocation (Variables|Default|GetTarget)) (Transformation|GetActorLocation)))))
  (Transformation|SetActorLocation (+ (Transformation|GetActorLocation (Variables|Default|GetFollowedPlayer)) (Variables|Default|GetPositionOffset)) false false))

(fn ConstructionScript)