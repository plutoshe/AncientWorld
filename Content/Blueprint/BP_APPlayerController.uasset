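; BP_APPlayerController is a player controller that creates the HUD and highlights interactable items under the cursor.
; BeginPlay creates the BP_HUD widget and adds it to the viewport.
; Each Tick, a complex visibility trace under the cursor shows the outline mesh of an enabled APInteractItemBase and stores it as the current hit.
; That outline clears only when the cursor hits no interact item, not when it moves directly onto another.
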(event EventBeginPlay
  (bind _returnvalue (UserInterface|CreateWidget "/Game/UI/BP_HUD.BP_HUD_C"))
  (bind _output_get (Variables|Default|SetHudWidget _returnvalue))
  (UserInterface|Viewport|AddtoViewport _output_get 0))

(event EventTick
  (params (DeltaSeconds :type Float%20%28single-precision%29))
  (bind _asapinteract_item_base (Utilities|Casting|CastToAPInteractItemBase (.hitactor (.HitResult (Game|Player|GetHitResultUnderCursorbyChannel "TraceTypeQuery1" true))))
    (:then
      (if (not (Variables|/Script/AncientWorld.APInteractItemBase|Getm_bInteractDisabled _asapinteract_item_base))
        (if (not (Variables|/Script/AncientWorld.APInteractItemBase|Getm_bHasOutline _asapinteract_item_base))
          (Variables|Default|Setm_CurrentHitItem _asapinteract_item_base)
          (Rendering|SetVisibility (Variables|/Script/AncientWorld.APInteractItemBase|GetOutlineMesh _asapinteract_item_base) true false)
          (Variables|/Script/AncientWorld.APInteractItemBase|Setm_bHasOutline _asapinteract_item_base true))))
    (:CastFailed
      (Utilities|IsValid (Variables|Default|Getm_CurrentHitItem)
        (:Is%20Valid
          (Rendering|SetVisibility (Variables|/Script/AncientWorld.APInteractItemBase|GetOutlineMesh (Variables|Default|Getm_CurrentHitItem)) false false)
          (Variables|/Script/AncientWorld.APInteractItemBase|Setm_bHasOutline (Variables|Default|Getm_CurrentHitItem) false)
          (Variables|Default|Setm_CurrentHitItem 0))))))

(fn ConstructionScript)